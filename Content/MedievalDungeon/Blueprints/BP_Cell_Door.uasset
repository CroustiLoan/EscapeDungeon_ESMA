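; Cell door Blueprint for the medieval dungeon that swings open and shut or plays a locked animation on Interaction.
; When locked, a separate timeline replays from the start; otherwise IsClosed toggles and RotationDoor plays forward or reverses.
; Both timelines drive the door mesh's yaw, scaled by RotationAngle.
; The construction script sets the initial rotation and RotationDoor time from IsClosed, so doors can start open.
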(event EventBeginPlay)

(event EventInteraction
  (if (Variables|Default|GetIsLocked)
    (bind _rotationvalue (Timeline|Timeline PlayFromStart)
      (:Update
        (Transformation|SetRelativeRotation (Variables|Default|GetSM_Cell_Door) (Math|Rotator|MakeRotator 0.0 0.0 (* _rotationvalue (Variables|Default|GetRotationAngle) -1.0)) false false)))
    (elif (Variables|Default|GetIsClosed)
      (Variables|Default|SetIsClosed false)
      (bind _rotationvalue_2 (Timeline|RotationDoor Play)
        (:Update
          (Transformation|SetRelativeRotation (Variables|Default|GetSM_Cell_Door) (Math|Rotator|MakeRotator 0.0 0.0 (* _rotationvalue_2 (Variables|Default|GetRotationAngle) -1.0)) false false)))
      (else
        (Variables|Default|SetIsClosed true)
        (Timeline|RotationDoor Reverse)))))

(fn ConstructionScript
  (Transformation|SetRelativeRotation (Variables|Default|GetSM_Cell_Door) (Math|Rotator|MakeRotator 0.0 0.0 (select (Variables|Default|GetIsClosed) 1.8e+02 (+ (Variables|Default|GetRotationAngle) 1.8e+02))) false false)
  (Transformation|SetRelativeRotation (Variables|Default|GetSM_Cell_Door) (Math|Rotator|MakeRotator 0.0 0.0 (select (Variables|Default|GetIsClosed) 0.0 (* (Variables|Default|GetRotationAngle) -1.0))) false false)
  (Components|Timeline|SetNewTime (Variables|Default|GetRotationDoor) (select (Variables|Default|GetIsClosed) 0.0 1.0)))